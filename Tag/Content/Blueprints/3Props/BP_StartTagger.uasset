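; BP_StartTagger is a one-use trigger prop that assigns the tagger role to a player.
; When a VRPawn with the Player tag enters or leaves its TagStarter collision, it calls BecomeTagger on that pawn.
; After the player leaves, the prop waits briefly and destroys itself.
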(event `self.Tag Starter.OnComponentBeginOverlap`
  (params (OverlappedComponent :type "PrimitiveComponent Object Reference") (OtherActor :type "Actor Object Reference") (OtherComp :type "PrimitiveComponent Object Reference") (OtherBodyIndex :type Integer) (bFromSweep :type Boolean) (SweepResult :type "HitResult Structure (by ref)"))
  ;[1 1 1] Make Person Tagger
  (if (`self.ActorHasTag` OtherActor "Player")
    (bind _asvrpawn (cast `/Game/Blueprints/1Players/VRPawn` OtherActor))
    (`/Game/Blueprints/1Players/VRPawn.Become Tagger` _asvrpawn)))

(event `self.Tag Starter.OnComponentEndOverlap`
  (params (OverlappedComponent :type "PrimitiveComponent Object Reference") (OtherActor :type "Actor Object Reference") (OtherComp :type "PrimitiveComponent Object Reference") (OtherBodyIndex :type Integer))
  ;[1 1 1] Make Person Tagger
  (if (`self.ActorHasTag` OtherActor "Player")
    (bind _asvrpawn (cast `/Game/Blueprints/1Players/VRPawn` OtherActor))
    (`/Game/Blueprints/1Players/VRPawn.Become Tagger` _asvrpawn)
    (`KismetSystemLibrary.Delay` 0.5)
    (`self.K2_DestroyActor`)))

(fn `UserConstructionScript`)