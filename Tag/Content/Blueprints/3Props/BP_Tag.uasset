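; BP_Tag is a prop that passes the tagger role in a VR game of tag when its Box overlaps a player.
; If the touched VRPawn is not the tagger, every VRPawn becomes a runner, then after a one-second delay the touched pawn becomes the tagger.
; Touching a pawn that is already the tagger only plays a 2D failure sound.
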(event `self.Box.OnComponentBeginOverlap`
  (params (OverlappedComponent :type "PrimitiveComponent Object Reference") (OtherActor :type "Actor Object Reference") (OtherComp :type "PrimitiveComponent Object Reference") (OtherBodyIndex :type Integer) (bFromSweep :type Boolean) (SweepResult :type "HitResult Structure (by ref)"))
  ;[1 1 1] Tag Other Player When Hit
  (if (`self.ActorHasTag` OtherActor "Player")
    (bind _asvrpawn (cast `/Game/Blueprints/1Players/VRPawn` OtherActor))
    (set `self.Player Being Tagged` _asvrpawn)
    (if (not (`/Game/Blueprints/1Players/VRPawn.Tagger?` _asvrpawn))
      (bind _outactors (`GameplayStatics.GetAllActorsOfClass` "/Game/Blueprints/1Players/VRPawn.VRPawn_C"))
      (for _array_element _outactors
        (`/Game/Blueprints/1Players/VRPawn.Become Runner` _array_element))
      (`KismetSystemLibrary.Delay` 1.0)
      (`/Game/Blueprints/1Players/VRPawn.Become Tagger` (`self.Player Being Tagged`))
      (else
        (`GameplayStatics.PlaySound2D` "/Engine/EditorSounds/Notifications/CompileFailed_Cue.CompileFailed_Cue" 1.0 1.0 0.0 null null)))))

(fn `UserConstructionScript`)